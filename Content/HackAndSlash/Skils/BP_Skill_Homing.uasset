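; Homing projectile skill actor that seeks a nearby object and destroys itself shortly after overlapping any actor.
; Each tick a sphere trace around the Arrow component picks a target of one object type, with debug drawing left on.
; The Arrow smoothly turns toward that target using only X and Y coordinates, then moves forward at Speed without sweeping.
; The last target is kept when the trace finds nothing.
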(event EventBeginPlay
  (|CallParentFunction) ; This node is disabled and will not be called.\nDrag off pins to build functionality.
)

(event Collision|EventActorBeginOverlap
  (params (OtherActor :type Actor%20Object%20Reference))
  (Utilities|Time|SetTimerbyFunctionName 0 "CallDestroy" 0.1))

(event EventTick
  (params (DeltaSeconds :type Float%20%28single-precision%29))
  (CallFunction|FindTarget)
  (CallFunction|RotatetoTarget DeltaSeconds)
  (CallFunction|MoveForward DeltaSeconds))

(fn ConstructionScript
  (|CallParentFunction))

(fn MoveForward
  (params (DeltaSeconds :type Float%20%28double-precision%29))
  (bind _arrow (Variables|Default|GetArrow))
  (Transformation|AddWorldOffset _arrow (* (Math|Vector|GetForwardVector _arrow) (* DeltaSeconds (Variables|Default|GetSpeed))) false false))

(fn RotatetoTarget
  (params (DeltaSeconds :type Float%20%28double-precision%29))
  (bind _arrow (Variables|Default|GetArrow))
  (bind _returnvalue (Transformation|GetWorldLocation _arrow))
  (bind _target (Variables|Default|GetTarget)
    (:then
      (Transformation|SetWorldRotation (Variables|Default|GetArrow) (Math|Interpolation|RInterpTo (Transformation|GetWorldRotation _arrow) (Math|Rotator|FindLookatRotation (Math|Vector|MakeVector (.x _returnvalue) (.y _returnvalue) 0.0) (Math|Vector|MakeVector (.x (Transformation|GetActorLocation _target)) (.y (Transformation|GetActorLocation _target)) 0.0)) DeltaSeconds 1e+01) false false))
    (:else)))

(fn FindTarget
  (bind _arrow (Variables|Default|GetArrow))
  (bind _returnvalue (Transformation|GetWorldLocation _arrow))
  (bind (_outhit _returnvalue_2) (Collision|SphereTraceForObjects _returnvalue _returnvalue 1e+03 (Utilities|Array|MakeArray "ObjectTypeQuery7") false 0 "ForOneFrame"))
  (if _returnvalue_2
    (Variables|Default|SetTarget (.HitActor (Collision|BreakHitResult _outhit)))))

(fn CallDestroy
  (Actor|DestroyActor))