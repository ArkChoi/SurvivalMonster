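; BP_HSGameMode is the hack-and-slash game mode that drives the match through Ready, Play and End states held in BP_HSGameState.
; BeginPlay sets Ready, and Tick switches to Play once the game state's accumulated time passes a short fixed delay.
; During Play, every Tick binds to the death dispatcher on the player hero's StatComponent.
; BindDeath, apparently the handler for that dispatcher, moves the game to End.
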(event EventBeginPlay
  (bind _asbp_hsgame_state (Utilities|Casting|CastToBP_HSGameState (Game|GetGameState)))
  (Default|ChangeGameState _asbp_hsgame_state "NewEnumerator1"))

(event EventTick
  (params (DeltaSeconds :type Float%20%28single-precision%29))
  (bind _asbp_hsgame_state (Utilities|Casting|CastToBP_HSGameState (Game|GetGameState)))
  (switch Utilities|FlowControl|Switch|SwitchonEN_GameState (Variables|/Game/HackAndSlash/GameMode/BP_HSGameState.BP_HSGameState_C|GetGameState _asbp_hsgame_state)
    (:NewEnumerator1
      (CallFunction|UpdateReady (Variables|/Game/HackAndSlash/GameMode/BP_HSGameState.BP_HSGameState_C|GetTotalDeltaSeconds _asbp_hsgame_state) _asbp_hsgame_state))
    (:NewEnumerator2
      (CallFunction|UpdatePlay))))

(fn ConstructionScript)

(fn UpdateReady
  (params (TotalDeltaSeconds :type Float%20%28double-precision%29) (GameState :type BP%20HS%20Game%20State%20Object%20Reference))
  (if (> TotalDeltaSeconds 6.0)
    (Default|ChangeGameState GameState "NewEnumerator2")))

(fn BindDeath
  (bind _asbp_hsgame_state (Utilities|Casting|CastToBP_HSGameState (Game|GetGameState)))
  (Default|ChangeGameState _asbp_hsgame_state "NewEnumerator3"))

(fn UpdatePlay
  (bind _asbp_hero (Utilities|Casting|CastToBP_Hero (Pawn|GetControlledPawn (Game|GetPlayerController 0))))
  (EventDispatchers|BindEventtoEventDispatcherDeath (Variables|/Game/HackAndSlash/GameMode/BP_Hero.BP_Hero_C|GetStatComponent _asbp_hero) (EventDispatchers|CreateEvent :!event BindDeath)))